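; RadiationStorm_BP is a timed radiation storm event actor that takes effect as soon as it spawns.
; On BeginPlay it dims the level's Directional Light and doubles the player BP_TopDownVacaCharacter's radiation multiplier (RadMult).
; After a ten-second delay it raises the light intensity to a fixed brighter value, resets the multiplier to one and destroys itself.
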(event `self.ReceiveBeginPlay`
  (bind _returnvalue (`GameplayStatics.GetActorOfClass` "/Script/Engine.DirectionalLight"))
  (`LightComponent.SetIntensity` (`Light.LightComponent` _returnvalue) 1.5)
  (bind _asbp_top_down_vaca_character (cast `/Game/Developers/SanGameDev/BP_TopDownVacaCharacter` (`GameplayStatics.GetPlayerCharacter` 0)))
  (set `/Game/Developers/SanGameDev/BP_TopDownVacaCharacter.RadMult` 2 _asbp_top_down_vaca_character)
  (`KismetSystemLibrary.Delay` 10.0)
  (bind _returnvalue_2 (`GameplayStatics.GetActorOfClass` "/Script/Engine.DirectionalLight"))
  (`LightComponent.SetIntensity` (`Light.LightComponent` _returnvalue_2) 3.0)
  (set `/Game/Developers/SanGameDev/BP_TopDownVacaCharacter.RadMult` 1 _asbp_top_down_vaca_character)
  (`self.K2_DestroyActor`))

(fn `UserConstructionScript`)