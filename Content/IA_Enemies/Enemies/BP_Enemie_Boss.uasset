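; Boss enemy for the horde game mode that attacks the player in an endless loop and, when its health runs out, destroys itself and restarts the horde.
; A random looping MultiGate picks among a radial blast, a cone blast and a knife spawn, each telegraphed by briefly showing a shape.
; The radial blast damages by distance check, while the cone blast relies on a flag set by overlap events.
; Standby and wake-up functions only toggle visibility.
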(event `self.ReceiveBeginPlay`
  (`parent.ReceiveBeginPlay`)
  (bind _asbp_top_down_vaca_character (cast `/Game/Developers/SanGameDev/BP_TopDownVacaCharacter` (`GameplayStatics.GetPlayerCharacter` 0)))
  (set `self.Player` _asbp_top_down_vaca_character)
  (`self.Boss Attacks`))

(event `self.ReceiveTick`
  (params (DeltaSeconds :type "Float (single-precision)"))
  (`parent.ReceiveTick` DeltaSeconds)
  (if (<= (`self.currentHealth`) 0.0)
    (`self.K2_DestroyActor`)
    (bind _asbp_top_down_game_mode_horde (cast `/Game/HordeSystem/BP_TopDownGameMode_Horde` (`GameplayStatics.GetGameMode`)))
    (`/Game/HordeSystem/BP_TopDownGameMode_Horde.RestartHorde` _asbp_top_down_game_mode_horde)))

(event `self.ConeAttack.OnComponentBeginOverlap`
  (params (OverlappedComponent :type "PrimitiveComponent Object Reference") (OtherActor :type "Actor Object Reference") (OtherComp :type "PrimitiveComponent Object Reference") (OtherBodyIndex :type Integer) (bFromSweep :type Boolean) (SweepResult :type "HitResult Structure (by ref)"))
  (cast `/Game/Developers/SanGameDev/BP_TopDownVacaCharacter` OtherActor)
  (set `self.InConeRange` true))

(event `self.ConeAttack.OnComponentEndOverlap`
  (params (OverlappedComponent :type "PrimitiveComponent Object Reference") (OtherActor :type "Actor Object Reference") (OtherComp :type "PrimitiveComponent Object Reference") (OtherBodyIndex :type Integer))
  (cast `/Game/Developers/SanGameDev/BP_TopDownVacaCharacter` OtherActor)
  (set `self.InConeRange` false))

(event `Boss Attacks`
  (`|MultiGate` true true 3
    (:`Out 0`
      (`SceneComponent.SetVisibility` (`self.Sphere1`) true false)
      (`KismetSystemLibrary.Delay` 2.0)
      (`SceneComponent.SetVisibility` (`self.Sphere1`) false false)
      (`GameplayStatics.SpawnEmitterAtLocation` "/Game/StarterContent/Particles/P_Explosion.P_Explosion" (`self.K2_GetActorLocation`) (struct) (2.0 2.0 2.0))
      (if (<= (`KismetMathLibrary.Vector_Distance` (`self.K2_GetActorLocation`) (`self.K2_GetActorLocation` (`self.Player`))) 350.0)
        (`/Game/Developers/SanGameDev/BP_TopDownVacaCharacter.TakeDamage` (`self.Player`) 10.0))
      (`KismetSystemLibrary.Delay` 2.0)
      (`self.Boss Attacks`))
    (:`Out 1`
      (`SceneComponent.SetVisibility` (`self.ConeAttack`) true false)
      (`KismetSystemLibrary.Delay` 2.0)
      (`SceneComponent.SetVisibility` (`self.ConeAttack`) false false)
      (`GameplayStatics.SpawnEmitterAtLocation` "/Game/StarterContent/Particles/P_Explosion.P_Explosion" (`SceneComponent.K2_GetComponentLocation` (`self.ConeAttack`)) (struct) (2.0 2.0 2.0))
      (if (`self.InConeRange`)
        (`/Game/Developers/SanGameDev/BP_TopDownVacaCharacter.TakeDamage` (`self.Player`) 10.0))
      (`KismetSystemLibrary.Delay` 2.0)
      (`self.Boss Attacks`))
    (:`Out 2`
      (`SceneComponent.SetVisibility` (`self.Cube`) true false)
      (`KismetSystemLibrary.Delay` 2.0)
      (`SceneComponent.SetVisibility` (`self.Cube`) false false)
      (`|SpawnActorFromClass` "/Game/IA_Enemies/Enemies/BP_Boss_Knife.BP_Boss_Knife_C" (`SceneComponent.K2_GetComponentToWorld` (`self.Cube`)) "Undefined" "MultiplyWithRoot" null null)
      (`KismetSystemLibrary.Delay` 2.0)
      (`self.Boss Attacks`))))

(fn `StandbyFunction`
  (`self.SetActorHiddenInGame` true))

(fn `UserConstructionScript`
  (`parent.UserConstructionScript`))

(fn `WakeUpFunction`
  (`self.SetActorHiddenInGame` false))