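; BP_Enemie_Ranged is a ranged enemy that pursues the player and fires BP_Enemie_Bullet projectiles.
; Each Tick destroys it at zero health or issues AI MoveTo toward the player, stopping at a standoff radius.
; When a distance check passes, it turns to face the player and, after a Delay that paces fire, spawns a bullet at its Cube component's transform.
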(event `self.ReceiveTick`
  (params (DeltaSeconds :type "Float (single-precision)"))
  (bind _returnvalue (`GameplayStatics.GetPlayerCharacter` 0))
  (if (<= (`self.currentHealth`) 0.0)
    (`self.K2_DestroyActor`)
    (else
      (`|AIMoveTo` self (0.0 0.0 0.0) (`GameplayStatics.GetPlayerCharacter` 0) 500.0
        (:`then`
          (if (<= (`self.GetDistanceTo` null) 700.0)
            (`/Engine/EditorBlueprintResources/StandardMacros.IsValid` _returnvalue
              (:`Is Valid`
                (`self.K2_SetActorRotation` (`KismetMathLibrary.FindLookAtRotation` (`self.K2_GetActorLocation`) (`self.K2_GetActorLocation` _returnvalue))))
              (:`Is Not Valid`
                _))
            (`KismetSystemLibrary.Delay` 2.0)
            (`|SpawnActorFromClass` "/Game/IA_Enemies/Enemies/BP_Enemie_Bullet.BP_Enemie_Bullet_C" (`SceneComponent.K2_GetComponentToWorld` (`self.Cube`)) "Undefined" "MultiplyWithRoot" null null)))))))

(fn `UserConstructionScript`
  (`parent.UserConstructionScript`))