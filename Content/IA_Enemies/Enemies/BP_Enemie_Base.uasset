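; Base enemy for a top-down game that chases the player and may drop a pickup when destroyed.
; Tick reissues AI Move To toward the player every frame, or destroys the enemy once health, lowered through DealDamage, runs out.
; Capsule hits on the player character call TakeDamage with zero, apparently a placeholder.
; On destruction, nested coin flips leave nothing half the time, otherwise a health, RadAway or random weapon pickup.
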(event `self.ReceiveBeginPlay`
  (set `self.currentHealth` (`self.maxHealth`)))

(event `self.ReceiveTick`
  (params (DeltaSeconds :type "Float (single-precision)"))
  (if (<= (`self.currentHealth`) 0.0)
    (`self.K2_DestroyActor`)
    (else
      (`|AIMoveTo` self (0.0 0.0 0.0) (`GameplayStatics.GetPlayerCharacter` 0) 0.0 true))))

(event `self.CapsuleComponent.OnComponentHit`
  (params (HitComponent :type "PrimitiveComponent Object Reference") (OtherActor :type "Actor Object Reference") (OtherComp :type "PrimitiveComponent Object Reference") (NormalImpulse :type "Vector Structure") (Hit :type "HitResult Structure (by ref)"))
  (bind _asbp_top_down_vaca_character (cast `/Game/Developers/SanGameDev/BP_TopDownVacaCharacter` OtherActor))
  ;[1 1 1] Aqui va hacer daño
  (`/Game/Developers/SanGameDev/BP_TopDownVacaCharacter.TakeDamage` _asbp_top_down_vaca_character 0.0))

(event `self.ReceiveDestroyed`
  (bind _deathposition (`self.deathPosition`))
  (bind _deathposition_2 (`self.deathPosition`))
  (set `self.deathPosition` (`self.GetTransform`))
  (if (`KismetMathLibrary.RandomBool`)
    (if (`KismetMathLibrary.RandomBool`)
      (if (`KismetMathLibrary.RandomBool`)
        (`|SpawnActorFromClass` "/Game/CarlosCarpeta/Blueprints/PickUps/PickUpHealth_BP.PickUpHealth_BP_C" _deathposition "Undefined" "MultiplyWithRoot" null null)
        (else
          (`|SpawnActorFromClass` "/Game/CarlosCarpeta/Blueprints/PickUps/PickUpRadAway_BP.PickUpRadAway_BP_C" _deathposition "Undefined" "MultiplyWithRoot" null null)))
      (else
        (switch `int` (`KismetMathLibrary.RandomIntegerInRange` 0 2)
          (:`0`
            (`|SpawnActorFromClass` "/Game/CarlosCarpeta/Blueprints/PickUps/PickUpShotgun_BP.PickUpShotgun_BP_C" _deathposition_2 "Undefined" "MultiplyWithRoot" null null))
          (:`1`
            (`|SpawnActorFromClass` "/Game/CarlosCarpeta/Blueprints/PickUps/PickUpChainSaw_BP.PickUpChainSaw_BP_C" _deathposition_2 "Undefined" "MultiplyWithRoot" null null))
          (:`2`
            (`|SpawnActorFromClass` "/Game/CarlosCarpeta/Blueprints/PickUps/PickUpGranade_BP.PickUpGranade_BP_C" _deathposition_2 "Undefined" "MultiplyWithRoot" null null)))))))

(fn `DealDamage`
  (params (DamageToDeal :type "Float (double-precision)"))
  (bind _output_get (set `self.currentHealth` (- (`self.currentHealth`) DamageToDeal)))
  (`KismetSystemLibrary.PrintText` (`|FormatText` "Taken Damage, current health: {0}" _output_get)))

(fn `UserConstructionScript`)