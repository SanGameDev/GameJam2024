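; Extraction zone actor for the horde mode that decides whether the player wins or loses.
; On BeginPlay it starts a three-minute timer that shows the Game Over widget on expiry, adds a timer HUD and attaches a guide arrow to the player.
; Player overlap starts a five-second delay, then opens the End level and pauses if the player is inside at that moment, without checking for continuous presence.
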(event `self.ReceiveBeginPlay`
  (bind _returnvalue (`GameplayStatics.GetPlayerCharacter` 0))
  (bind _returnvalue_2 (`KismetSystemLibrary.K2_SetTimerDelegate` (delegate `Extract`) 180.0)) ; Three minutes before you lose
  (set `self.ExtractionTimer` _returnvalue_2)
  (bind _returnvalue_3 (`|GenericCreateObject` "/Game/CarlosCarpeta/Blueprints/Widgets/Timer_WG.Timer_WG_C"))
  (`UserWidget.AddToViewport` _returnvalue_3 0)
  (bind _returnvalue_4 (`|SpawnActorFromClass` "/Game/HordeSystem/BP_GuideArrow.BP_GuideArrow_C" (`KismetMathLibrary.MakeTransform` (`self.K2_GetActorLocation` _returnvalue)) "Undefined" "MultiplyWithRoot" null null))
  (`self.K2_AttachToActor` _returnvalue_4 _returnvalue "None" "KeepRelative" "KeepRelative" "KeepRelative" true)
  (set `self.GuideArrow` _returnvalue_4))

(event `Extract`
  ;[1 1 1] Lose process
  (bind _returnvalue (`|CreateWidget` "/Game/CarlosCarpeta/Blueprints/Widgets/GameOverUI_WG.GameOverUI_WG_C"))
  (`UserWidget.AddToViewport` _returnvalue 0))

(event `self.ReceiveActorBeginOverlap`
  (params (OtherActor :type "Actor Object Reference"))
  (cast `/Game/Developers/SanGameDev/BP_TopDownVacaCharacter` OtherActor)
  (set `self.PlayerPresent` true)
  (`KismetSystemLibrary.PrintString` "PlayerInRange")
  (`KismetSystemLibrary.Delay` 5.0) ; Make display for this
  (if (`self.PlayerPresent`)
    (`self.WinGame`)
    (else
      (`KismetSystemLibrary.PrintString` "Player out of bounds"))))

(event `self.ReceiveActorEndOverlap`
  (params (OtherActor :type "Actor Object Reference"))
  (cast `/Game/Developers/SanGameDev/BP_TopDownVacaCharacter` OtherActor)
  (set `self.PlayerPresent` false))

(event `WinGame`
  (`GameplayStatics.OpenLevel` "End")
  (`KismetSystemLibrary.PrintString` "Win Game")
  (`GameplayStatics.SetGamePaused` true))

(fn `UserConstructionScript`)